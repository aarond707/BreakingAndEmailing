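; BP_Doors is a door that swings open while an FPSController actor is inside its Box volume and closes when none remains.
; Tick polls the box overlaps every frame to play or reverse the OpenAndCloseDoor timeline.
; The timeline's Rotation track is added to the world yaw captured at BeginPlay, and roll and pitch are set to zero.
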(event EventBeginPlay
  (bind _output_get (Variables|Default|SetstartRotation (.yaw (Transformation|GetWorldRotation (Variables|Default|GetDoor))))))

(event EventTick
  (params (DeltaSeconds :type Float%20%28single-precision%29))
  (if (not (== (Utilities|Array|Length (Collision|GetOverlappingActors (Variables|Default|GetBox) "/Game/Blueprints/FPSController.FPSController_C" :!class /Script/Engine.PrimitiveComponent)) 0))
    ;[1 1 1] Animation for door opening and closing
    (bind _rotation (Timeline|openAndCloseDoor Play)
      (:Update
        (Transformation|SetWorldRotation (Variables|Default|GetDoor) (Math|Rotator|MakeRotator 0.0 0.0 (+ _rotation (stale EventBeginPlay _output_get))) false false)))
    (else
      (Timeline|openAndCloseDoor Reverse))))

(fn ConstructionScript)